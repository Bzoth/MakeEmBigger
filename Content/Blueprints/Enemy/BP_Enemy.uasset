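; Enemy pawn Blueprint that supplies an ordered sequence of patrol locations across two rooms, starting in RoomA.
; GetNewLocation returns the current point of the active room array and advances the index; no movement logic lives here.
; When a room's points run out, NewRoom resets the index and switches between RoomA and RoomB in a loop, and the lookup retries recursively.
; BeginPlay also turns off controller yaw rotation.
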(event EventBeginPlay
  (Variables|Default|SetbUseControllerRotationYaw false)
  (Variables|Default|SetCurrentRoom (Variables|Default|GetRoomA)))

(fn ConstructionScript)

(fn GetNewLocationinRoom
  (if (>= (Variables|Default|GetPointIndex) (Utilities|Array|Length (Variables|Default|GetCurrentRoom)))
    (CallFunction|NewRoom)
    (bind _point (CallFunction|GetNewLocationinRoom))
    (return _point)
    (else
      (return (Utilities|Array|Get(acopy) (Variables|Default|GetCurrentRoom) (Variables|Default|GetPointIndex))))))

(fn GetNewLocation
  (bind _point (CallFunction|GetNewLocationinRoom))
  (Math|Integer|IncrementInt (Variables|Default|GetPointIndex)
    (:%20%20
      (return _point))))

(fn NewRoom
  (Variables|Default|SetPointIndex 0)
  (Math|Integer|IncrementInt (Variables|Default|GetRoomIndex)
    (:%20%20
      (Variables|Default|SetCurrentRoom (CallFunction|IndextoRoom))
      (return))))

(fn IndextoRoom
  (if (> (Variables|Default|GetRoomIndex) 1)
    (Variables|Default|SetRoomIndex 0))
  (return (Utilities|Select :Index (Variables|Default|GetRoomIndex) :Option%200 (Variables|Default|GetRoomA) :Option%201 (Variables|Default|GetRoomB))))