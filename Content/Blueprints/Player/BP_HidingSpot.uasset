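; BP_HidingSpot is a hiding spot actor that tracks whether the player has used it.
; The first overlap by an actor tagged Player sets Used and switches the Cube to a red material.
; Nothing in the file resets Used, so each spot triggers only once.
; IsUsed reports that state as one of two enum values.
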(event Collision|EventActorBeginOverlap
  (params (OtherActor :type Actor%20Object%20Reference))
  (if (not (Variables|Default|GetUsed))
    (if (Actor|ActorHasTag OtherActor "Player")
      (Variables|Default|SetUsed true)
      (Rendering|Material|SetMaterial (Variables|Default|GetCube) 0 "/Game/Assets/Materials/M_Red.M_Red"))))

(fn ConstructionScript)

(fn IsUsed
  (return (select (Variables|Default|GetUsed) "NewEnumerator1" "NewEnumerator0")))